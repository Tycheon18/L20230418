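; BP_P38 is a player-controllable P-38 plane that flies constantly forward along its own forward vector.
; Each Tick moves it by MoveSpeed scaled by delta time, without sweep, and spins the Left and Right propellers through a shared PropellerRotate function.
; Pitch and Roll axis inputs are clamped and applied as world-space rotation deltas, not scaled by frame time.
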(event EventTick
  (params (DeltaSeconds :type Float%20%28single-precision%29))
  (Utilities|FlowControl|Sequence
    (:then_0
      (Transformation|AddActorWorldOffset (* (Transformation|GetActorForwardVector) (* (Variables|Default|GetMoveSpeed) (Utilities|Time|GetWorldDeltaSeconds)))))
    (:then_1
      (CallFunction|PropellerRotate (Variables|Default|GetLeft)))
    (:then_2
      (CallFunction|PropellerRotate (Variables|Default|GetRight)))))

(event Input|AxisEvents|InputAxisPitch
  (params (AxisValue :type Float%20%28single-precision%29))
  (Class|Actor|AddActorWorldRotation (Math|Rotator|MakeRotator 0.0 (Math|Float|Clamp(Float) AxisValue -1.0) 0.0)))

(event Input|AxisEvents|InputAxisRoll
  (params (AxisValue :type Float%20%28single-precision%29))
  (Class|Actor|AddActorWorldRotation (Math|Rotator|MakeRotator (Math|Float|Clamp(Float) AxisValue -1.0) 0.0 0.0)))

(fn ConstructionScript)

(fn PropellerRotate
  (params (Propeller :type Scene%20Component%20Object%20Reference))
  (Transformation|AddRelativeRotation Propeller (Math|Rotator|MakeRotator (* (Variables|Default|GetPropellerRotationSpeed) (Utilities|Time|GetWorldDeltaSeconds)) 0.0 0.0) false false))